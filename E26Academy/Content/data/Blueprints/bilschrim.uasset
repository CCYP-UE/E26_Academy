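; Screen actor that runs a looping slideshow of three images on its Bildschrim component.
; From BeginPlay, a self-looping 10-second delay advances a counter that selects the next texture and wraps after the third.
; Each pass creates a new dynamic material instance from Bild_Inst on the second material slot and sets its Video_textur parameter to that image.
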(event EventBeginPlay
  (Variables|Default|SetTexture_Count 0)
  (Utilities|FlowControl|Delay 1e+01 :!label _label)
  (bind _returnvalue (Rendering|Material|CreateDynamicMaterialInstance (Variables|Default|GetBildschrim) 1 "/Game/data/Meshs/Bildschrim/bild_Inst.bild_Inst" :!class /Script/Engine.PrimitiveComponent))
  (switch int (Variables|Default|GetTexture_Count)
    (:0
      (Variables|Default|SetTextur "/Game/data/Meshs/Bildschrim/Bild1.Bild1")
      (Variables|Default|SetTexture_Count 1))
    (:1
      (Variables|Default|SetTextur "/Game/data/Meshs/Bildschrim/Bild2.Bild2")
      (Variables|Default|SetTexture_Count 2))
    (:2
      (Variables|Default|SetTextur "/Game/data/Meshs/Bildschrim/Bild3.Bild3")
      (Variables|Default|SetTexture_Count 0)))
  (Rendering|Material|SetTextureParameterValue _returnvalue "Video_textur" (Variables|Default|GetTextur))
  (goto _label))

(event EventActorBeginOverlap
  (params (OtherActor :type Actor%20Object%20Reference)))

(event EventTick
  (params (DeltaSeconds :type Float%20%28single-precision%29)))

(fn ConstructionScript)